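; Game mode that runs a looping level structure, streaming numbered Loop sublevels in and out up to a final seventh loop.
; LoadLevel advances the loop counter, streams that level and plays a wake-up sequence before notifying the player pawn.
; UnloadLevel plays a sleep sequence, unloads the current loop and chains into LoadLevel when the sequence finishes.
; EndSequence plays the ending, unloads Loop7 and shows the end widget.
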(event Custom|On%20Finished
  ;[1 1 1] Load Stream Level
  ;;[1 1 1] Bind event on finished sequence to initialize player.
  (Class|BPIPlayer|BeginPlay(Message) (Game|Player|GetPlayerPawn 0)))

(event Custom|On%20Finished%20Sleep
  ;[1 1 1] Unload Stream Level
  ;;[1 1 1] Bind event on finished sequence to initialize next loop.
  (CallFunction|LoadLevel))

(event Custom|On%20Finished%20End
  ;[1 1 1] Play End Sequence
  ;;[1 1 1] Bind event on finished sequence to create end widget.
  (bind _returnvalue (UserInterface|CreateWidget "/Game/Widgets/WBP_End.WBP_End_C"))
  (UserInterface|Viewport|AddtoViewport _returnvalue 0))

(event EventBeginPlay)

(event EventTick
  (params (DeltaSeconds :type Float%20%28single-precision%29)))

(event EventUnloadLevel
  ;[1 1 1] Unload Stream Level
  (Utilities|FlowControl|Delay 1.5)
  ;;[1 1 1] Play Sleep Sequence
  (bind _returnvalue (Sequencer|Player|CreateLevelSequencePlayer "/Game/Maps/Sequences/Sleep.Sleep"))
  (Sequencer|Player|Play _returnvalue :!class /Script/MovieScene.MovieSceneSequencePlayer)
  ;;[1 1 1] Bind event on finished sequence to initialize next loop.
  (EventDispatchers|BindEventtoOnFinished _returnvalue (delegate Custom|On%20Finished%20Sleep))
  (Class|BPIPlayer|EndPlay(Message) (Game|Player|GetPlayerPawn 0))
  ;;[1 1 1] Unload current loop level.
  (Utilities|FlowControl|Delay 3.0)
  (Game|UnloadStreamLevel(byName) (Utilities|String|StringToName (Utilities|String|Append "Loop" (Utilities|String|ToString(Integer) (Variables|Default|GetCurrent%20Loop)))) false)
  (Audio|PlaySound2D "/Game/Assets/Sounds/MetaSounds/SFX/SFX_Teleport.SFX_Teleport" 1.0 1.0 0.0 0 0))

(event EventLoadLevel
  ;[1 1 1] Load Stream Level
  ;;[1 1 1] Load stream level based on current loop index.
  (bind _result (Math|Integer|IncrementInt (Variables|Default|GetCurrent%20Loop))
    (:%20%20
      (Game|LoadStreamLevel(byName) (Utilities|String|StringToName (Utilities|String|Append "Loop" (Utilities|String|ToString(Integer) _result))) true)
      ;;[1 1 1] Play Wake Up Sequence
      (bind _returnvalue (Sequencer|Player|CreateLevelSequencePlayer "/Game/Maps/Sequences/WakeUp.WakeUp"))
      (Sequencer|Player|Play _returnvalue :!class /Script/MovieScene.MovieSceneSequencePlayer)
      ;;[1 1 1] Bind event on finished sequence to initialize player.
      (EventDispatchers|BindEventtoOnFinished _returnvalue (delegate Custom|On%20Finished)))))

(event EventEndSequence
  ;[1 1 1] Play End Sequence
  ;;[1 1 1] Play Sleep Sequence
  (bind _returnvalue (Sequencer|Player|CreateLevelSequencePlayer "/Game/Maps/Sequences/End.End"))
  (Sequencer|Player|Play _returnvalue :!class /Script/MovieScene.MovieSceneSequencePlayer)
  ;;[1 1 1] Bind event on finished sequence to create end widget.
  (EventDispatchers|BindEventtoOnFinished _returnvalue (delegate Custom|On%20Finished%20End))
  (Class|BPIPlayer|EndPlay(Message) (Game|Player|GetPlayerPawn 0))
  ;;[1 1 1] Stop the loop 7 sound.
  (Utilities|FlowControl|Delay 5.0)
  (Game|UnloadStreamLevel(byName) "Loop7" false))

(fn ConstructionScript)

(fn GetIsFinalLoop
  (return (== (Variables|Default|GetCurrent%20Loop) 7)))